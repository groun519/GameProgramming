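; BP_MagicCircle_DecalMaker is a magic circle decal actor that spins continuously while facing straight down.
; Tick accumulates an angle scaled by delta time and RotateMultipler, wraps it past 360, and applies it as roll at -90 pitch, so the spin is around the vertical axis.
; A dynamic material branch that would tint the decal's BaseColor blue-violet is present but never runs.
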(event `self.ReceiveBeginPlay`)

(event `self.ReceiveTick`
  (params (DeltaSeconds :type "Float (single-precision)"))
  (if (> (`self.float`) 360.0)
    (set `self.float` (- (`self.float`) 360.0)))
  (bind _output_get (set `self.float` (+ (* DeltaSeconds (`self.RotateMultipler`)) (`self.float`))))
  (`self.K2_SetActorRotation` (`KismetMathLibrary.MakeRotator` _output_get -90.0)))

(fn `UserConstructionScript`)