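; BP_HandUpMagicCircle is a magic circle effect actor with a skeletal mesh, likely a raised hand, and a sphere that ends in an explosion.
; BeginPlay makes both meshes visible, then after a fixed delay spawns a large explosion emitter at the sphere's location.
; Tick calls Play on a timeline every frame, whose BallScale track drives the sphere's uniform world scale.
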(event `self.ReceiveBeginPlay`
  (`SceneComponent.SetVisibility` (`self.Sphere`) true false)
  (`SceneComponent.SetVisibility` (`self.SkeletalMesh`) true false)
  (`KismetSystemLibrary.Delay` 13.4)
  (`GameplayStatics.SpawnEmitterAtLocation` "/Game/StarterContent/Particles/P_Explosion.P_Explosion" (`SceneComponent.K2_GetComponentLocation` (`self.Sphere`)) (struct) (20.0 20.0 20.0)))

(event `self.ReceiveTick`
  (params (DeltaSeconds :type "Float (single-precision)"))
  (bind (_direction _ballscale) (`Timeline|Timeline_0` :`NewTime` DeltaSeconds)
    (:`Update`
      (`SceneComponent.SetWorldScale3D` (`self.Sphere`) (`KismetMathLibrary.MakeVector` _ballscale _ballscale _ballscale)))))

(fn `UserConstructionScript`)