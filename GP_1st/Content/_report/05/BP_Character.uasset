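; BP_Character is a key-driven character with W/S movement and A/D turning.
; W and S set DeltaLoc from the actor's forward vector and Speed, and A and D set RotZ, each cleared on release.
; Tick applies DeltaLoc as a swept local offset, though it derives from a world-space vector, without delta-time scaling.
; Tick also adds RotZ into DeltaRot and applies it as local rotation, so turn rate accumulates and persists after release.
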(event `Key|W`
  (params (Key :type "Key Structure"))
  ; MoveForward
  (:`Pressed`
    (set `self.DeltaLoc` (* (`self.GetActorForwardVector`) (`self.Speed`))))
  (:`Released`
    ; 속도를 0으로 설정해 움직이지 않게 함.
    (set `self.DeltaLoc` (0.0 0.0 0.0) :!label _label)))

(event `Key|S`
  (params (Key :type "Key Structure"))
  ; MoveForward
  (:`Pressed`
    (set `self.DeltaLoc` (`KismetMathLibrary.NegateVector` (* (`self.GetActorForwardVector`) (`self.Speed`)))))
  (:`Released`
    (goto _label)))

(event `Key|A`
  (params (Key :type "Key Structure"))
  ; MoveRight
  (:`Pressed`
    (set `self.RotZ` -1.0))
  (:`Released`
    (set `self.RotZ` 0.0 :!label _label_2)))

(event `self.ReceiveTick`
  (params (DeltaSeconds :type "Float (single-precision)"))
  ; Move
  (`self.K2_AddActorLocalOffset` (`self.DeltaLoc`) true)
  (bind _output_get (set `self.DeltaRot` (`KismetMathLibrary.MakeRotator` (.roll (`self.DeltaRot`)) (.pitch (`self.DeltaRot`)) (+ (.yaw (`self.DeltaRot`)) (`self.RotZ`)))))
  ; Rot
  (`self.K2_AddActorLocalRotation` _output_get))

(event `Key|D`
  (params (Key :type "Key Structure"))
  ; MoveRight
  (:`Pressed`
    (set `self.RotZ` 1.0))
  (:`Released`
    (goto _label_2)))

(fn `UserConstructionScript`)