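; BP_AppleSpawnner is a spawner actor that continuously creates BP_Apple actors around its own position.
; Each Tick makes a random roll with even odds of spawning an apple, so the spawn rate scales with frame rate.
; Apples take the spawner's transform, shifted randomly along world Y within plus or minus the Offset variable.
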(event `self.ReceiveTick`
  (params (DeltaSeconds :type "Float (single-precision)"))
  (bind _offset (`self.Offset`))
  (if (<= (`KismetMathLibrary.RandomIntegerInRange` 1 4) 2)
    (`|SpawnActorFromClass` "/Game/_WorkSpace/Blueprint/BP_Apple.BP_Apple_C" (`KismetMathLibrary.MakeTransform` (`KismetMathLibrary.MakeVector` (.x (.location (`self.GetTransform`))) (+ (.y (.location (`self.GetTransform`))) (`KismetMathLibrary.RandomFloatInRange` (* _offset -1.0) _offset)) (.z (.location (`self.GetTransform`)))) (.rotation (`self.GetTransform`)) (.scale (`self.GetTransform`))) "Undefined" "MultiplyWithRoot" null null)))

(fn `UserConstructionScript`)