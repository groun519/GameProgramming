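; BP_Apple is an apple actor that launches itself with a physics push when play begins.
; BeginPlay applies a randomly scaled forward force to its Sphere component at the actor location plus a Loc offset, then draws a debug sphere at that point.
; The NSquare helper multiplies a value by a power of ten through a countdown loop, but nothing in this file calls it.
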(event `self.ReceiveActorBeginOverlap`
  (params (OtherActor :type "Actor Object Reference")))

(event `self.ReceiveTick`
  (params (DeltaSeconds :type "Float (single-precision)")))

(event `self.ReceiveBeginPlay`
  (bind _returnvalue (+ (`self.Loc`) (`self.K2_GetActorLocation`)))
  (`PrimitiveComponent.AddForceAtLocation` (`self.Sphere`) (* (`self.GetActorForwardVector`) (* (`KismetMathLibrary.RandomFloatInRange` 0.01 0.02) 10000000.0)) _returnvalue "None")
  (`KismetSystemLibrary.DrawDebugSphere` _returnvalue 5.0))

(fn `NSquare`
  (params (SqaureNum :type Integer) (Multipler :type "Float (double-precision)"))
  (returns (ReturnValue :type "Float (double-precision)"))
  (locals (Val :type "Float (double-precision)") (Num :type Integer))
  (set `local.Num` SqaureNum)
  (set `local.Val` (* Multipler 1.0))
  (if (> (`local.Num`) 0) :!label _label
    (set `local.Val` (* (`local.Val`) 10.0))
    (`/Engine/EditorBlueprintResources/StandardMacros.DecrementInt` (`local.Num`)
      (:`  `
        (goto _label)))
    (else
      (return (`local.Val`)))))

(fn `UserConstructionScript`)